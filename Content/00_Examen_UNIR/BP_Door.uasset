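; BP_Door is a door driven by a set of linked buttons, currently reporting open or closed only as printed Spanish messages.
; On BeginPlay it binds each button's pressed-change event to a check that overwrites Allpressed per button, so only the last one decides the result.
; OpenDoor and CloseDoor play separate timelines, but the check never calls them and the left-door movement nodes are left unconnected.
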(event Custom|OpenDoor
  (bind _open (Timeline|TimelineOpen Play)))

(event Custom|CloseDoor
  (Timeline|TimelineClose Play))

(event Custom|ButtonsPressed
  (for _array_element (Variables|Default|GetButtons)
    (if (Variables|/Game/00_Examen_UNIR/BP_FloorButton.BP_FloorButton_C|GetPressed _array_element)
      (Variables|Default|SetAllpressed true)
      (else
        (Variables|Default|SetAllpressed false))))
  (if (Variables|Default|GetAllpressed)
    (Development|PrintString "La puerta se abre")
    (else
      (Development|PrintString "Esta cerrada"))))

(event EventBeginPlay
  (for _array_element (Variables|Default|GetButtons)
    (EventDispatchers|BindEventtoOnPressedChanged _array_element (delegate Custom|ButtonsPressed))))

(fn ConstructionScript)