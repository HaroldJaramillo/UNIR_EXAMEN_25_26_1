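; BP_FloorButton is an interactable floor button that the player toggles with E while inside its trigger box.
; Box overlap events set IsInside and enable or disable input from player controller 0, without checking which actor overlaps.
; E flips Pressed, but OnPressedChanged is called only on pressing, not on releasing.
; Debug strings print on entering, leaving and each toggle.
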(event OnComponentBeginOverlap(Box)
  (params (OverlappedComponent :type Primitive%20Component%20Object%20Reference) (OtherActor :type Actor%20Object%20Reference) (OtherComp :type Primitive%20Component%20Object%20Reference) (OtherBodyIndex :type Integer) (bFromSweep :type Boolean) (SweepResult :type Hit%20Result%20Structure%20%28by%20ref%29))
  (Variables|Default|SetIsInside true)
  (Input|EnableInput (Game|GetPlayerController 0))
  (Development|PrintString "Adentro"))

(event OnComponentEndOverlap(Box)
  (params (OverlappedComponent :type Primitive%20Component%20Object%20Reference) (OtherActor :type Actor%20Object%20Reference) (OtherComp :type Primitive%20Component%20Object%20Reference) (OtherBodyIndex :type Integer))
  (Variables|Default|SetIsInside false)
  (Input|DisableInput (Game|GetPlayerController 0))
  (Development|PrintString "Afuera"))

(event EventBeginPlay)

(event Input|KeyboardEvents|E
  (params (Key :type Key%20Structure :default "None"))
  (:Pressed
    (if (Variables|Default|GetPressed)
      (Variables|Default|SetPressed false)
      (Development|PrintString "E pulsada para despulsar")
      (else
        (Variables|Default|SetPressed true)
        (Default|CallOnPressedChanged)
        (Development|PrintString "E pulsada para pulsar")))))

(fn ConstructionScript)